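; Spline walker actor that rides along a chain of splines as a moving cart in what appears to be a puzzle.
; A timeline, rate-scaled by Duration and begun at StartOffset, drives position and rotation by distance along the current spline, starting on BeginPlay if Active.
; On finish, it continues onto the end hit box's NextSpline if IsInBox is set and that spline differs.
; Without a valid hit box, it marks itself finished.
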(event `self.ReceiveBeginPlay`
  (if (`self.Active`)
    (`self.MoveCart`)))

(event `MoveCart`
  (bind _endpointhitbox (`/Game/Blueprints/Spline/PipeSpline.EndPointHitBox` (`self.SplineReference`)))
  (bind _nextspline (`/Game/Blueprints/Spline/SplineEndHitBox.NextSpline` _endpointhitbox))
  (bind _returnvalue (`KismetMathLibrary.Lerp` 0.0 (`SplineComponent.GetSplineLength` (`/Game/Blueprints/Spline/PipeSpline.Spline` (`self.SplineReference`))) (`self.Alpha`)))
  (`TimelineComponent.SetPlayRate` (`self.Movement`) (/ 1.0 (`self.Duration`)))
  (`TimelineComponent.SetNewTime` (`self.Movement`) (`self.StartOffset`))
  (bind (_direction _alpha) (`Timeline|Movement`)
    (:`Update`
      (set `self.Alpha` _alpha)
      (`self.K2_SetActorLocationAndRotation` (`SplineComponent.GetLocationAtDistanceAlongSpline` (`/Game/Blueprints/Spline/PipeSpline.Spline` (`self.SplineReference`)) _returnvalue "World") (`SplineComponent.GetRotationAtDistanceAlongSpline` (`/Game/Blueprints/Spline/PipeSpline.Spline` (`self.SplineReference`)) _returnvalue "World")))
    (:`Finished`
      (if (`KismetSystemLibrary.IsValid` (`/Game/Blueprints/Spline/PipeSpline.EndPointHitBox` (`self.SplineReference`)))
        (if (`/Game/Blueprints/Spline/SplineEndHitBox.IsInBox` _endpointhitbox)
          (if (not (== _nextspline (`self.SplineReference`)))
            (set `self.SplineReference` _nextspline)
            (`self.MoveCart`)))
        (else
          (`KismetSystemLibrary.PrintString` "End Puzzle")
          (set `self.IsFinished` true))))))

(fn `UserConstructionScript`)