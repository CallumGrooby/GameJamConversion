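; Pushable object that GameCharacter can shove around by physics while in contact with its trigger volumes.
; Overlap begin on either the X-axis or Y-axis collision enables physics simulation on the Cube and sets the character's IsPushing flag.
; Overlap end on either volume turns simulation off and clears the flag, with no check on whether the other volume is still overlapped.
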(event `self.Y Axis Collision.OnComponentBeginOverlap`
  (params (OverlappedComponent :type "PrimitiveComponent Object Reference") (OtherActor :type "Actor Object Reference") (OtherComp :type "PrimitiveComponent Object Reference") (OtherBodyIndex :type Integer) (bFromSweep :type Boolean) (SweepResult :type "HitResult Structure (by ref)"))
  (bind _asgame_character (cast `/Game/Blueprints/Character/GameCharacter` OtherActor))
  (`PrimitiveComponent.SetSimulatePhysics` (`self.Cube`) true)
  (set `/Game/Blueprints/Character/GameCharacter.IsPushing` true _asgame_character))

(event `self.Y Axis Collision.OnComponentEndOverlap`
  (params (OverlappedComponent :type "PrimitiveComponent Object Reference") (OtherActor :type "Actor Object Reference") (OtherComp :type "PrimitiveComponent Object Reference") (OtherBodyIndex :type Integer))
  (bind _asgame_character (cast `/Game/Blueprints/Character/GameCharacter` OtherActor))
  (`PrimitiveComponent.SetSimulatePhysics` (`self.Cube`) false)
  (set `/Game/Blueprints/Character/GameCharacter.IsPushing` false _asgame_character))

(event `self.X Axis Collision.OnComponentBeginOverlap`
  (params (OverlappedComponent :type "PrimitiveComponent Object Reference") (OtherActor :type "Actor Object Reference") (OtherComp :type "PrimitiveComponent Object Reference") (OtherBodyIndex :type Integer) (bFromSweep :type Boolean) (SweepResult :type "HitResult Structure (by ref)"))
  (bind _asgame_character (cast `/Game/Blueprints/Character/GameCharacter` OtherActor))
  (`PrimitiveComponent.SetSimulatePhysics` (`self.Cube`) true)
  (set `/Game/Blueprints/Character/GameCharacter.IsPushing` true _asgame_character))

(event `self.X Axis Collision.OnComponentEndOverlap`
  (params (OverlappedComponent :type "PrimitiveComponent Object Reference") (OtherActor :type "Actor Object Reference") (OtherComp :type "PrimitiveComponent Object Reference") (OtherBodyIndex :type Integer))
  (bind _asgame_character (cast `/Game/Blueprints/Character/GameCharacter` OtherActor))
  (`PrimitiveComponent.SetSimulatePhysics` (`self.Cube`) false)
  (set `/Game/Blueprints/Character/GameCharacter.IsPushing` false _asgame_character))

(fn `UserConstructionScript`)