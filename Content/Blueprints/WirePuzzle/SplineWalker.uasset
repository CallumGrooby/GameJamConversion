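; Wire puzzle actor that rides along splines as a cart, starting on BeginPlay.
; A timeline scaled by Duration, starting at StartOffset, drives its position and rotation by distance along the current spline.
; At each end, the spline's EndPointHitBox either hands over a different next spline or, when not in its box, replays the current one.
; Without a hit box, it marks itself finished and has SplineManager unlock the door if the puzzle is complete.
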(event `self.ReceiveBeginPlay`
  (`self.MoveCart`))

(event `MoveCart`
  (bind _returnvalue (`KismetMathLibrary.Lerp` 0.0 (`SplineComponent.GetSplineLength` (`/Game/Blueprints/WirePuzzle/PipeSpline.Spline` (`self.SplineReference`))) (`self.Alpha`)))
  (`TimelineComponent.SetPlayRate` (`self.Movement`) (/ 1.0 (`self.Duration`)))
  (`TimelineComponent.SetNewTime` (`self.Movement`) (`self.StartOffset`))
  (bind (_direction _alpha) (`Timeline|Movement`)
    (:`Update`
      (set `self.Alpha` _alpha)
      (`self.K2_SetActorLocationAndRotation` (`SplineComponent.GetLocationAtDistanceAlongSpline` (`/Game/Blueprints/WirePuzzle/PipeSpline.Spline` (`self.SplineReference`)) _returnvalue "World") (`SplineComponent.GetRotationAtDistanceAlongSpline` (`/Game/Blueprints/WirePuzzle/PipeSpline.Spline` (`self.SplineReference`)) _returnvalue "World")))
    (:`Finished`
      (`self.SelectNext Spline`))))

(event `SelectNext Spline`
  (bind _endpointhitbox (`/Game/Blueprints/WirePuzzle/PipeSpline.EndPointHitBox` (`self.SplineReference`)))
  (bind _nextspline (`/Game/Blueprints/WirePuzzle/SplineEndHitBox.NextSpline` _endpointhitbox))
  (if (`KismetSystemLibrary.IsValid` (`/Game/Blueprints/WirePuzzle/PipeSpline.EndPointHitBox` (`self.SplineReference`)))
    (if (`/Game/Blueprints/WirePuzzle/SplineEndHitBox.IsInBox` _endpointhitbox)
      (if (not (== _nextspline (`self.SplineReference`)))
        (set `self.SplineReference` _nextspline)
        (`self.MoveCart`))
      (else
        (`KismetSystemLibrary.PrintString` "restart")
        (`self.MoveCart`)))
    (else
      (set `self.isFinished` true)
      (bind _returnvalue (`SplineManager.CheckIfPuzzleIsComplete` (`self.SplineManager`)))
      (if _returnvalue
        (`SplineManager.UnlockDoor` (`self.SplineManager`))))))

(fn `UserConstructionScript`)