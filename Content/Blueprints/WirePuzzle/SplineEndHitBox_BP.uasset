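; Trigger box for the wire puzzle, apparently at a spline end, that tracks whether a character has acted inside it.
; On overlap it flags the GameCharacter as in the box, takes it as owner and enables Tick logic.
; While enabled, Tick sets IsInBox through client and server events once the character plays an animation.
; Leaving the box clears both flags and stops the Tick logic.
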(event `self.ReceiveTick`
  (params (DeltaSeconds :type "Float (single-precision)"))
  (if (`self.ExecuteLogic`)
    (if (`/Game/Blueprints/Character/GameCharacter.IsPlayingAnimation` (`self.As Game Character`))
      (`self.SetIsInBox_Client` true)
      (`self.SetIsInBox_Server` true))))

(event `self.Box.OnComponentBeginOverlap`
  (params (OverlappedComponent :type "PrimitiveComponent Object Reference") (OtherActor :type "Actor Object Reference") (OtherComp :type "PrimitiveComponent Object Reference") (OtherBodyIndex :type Integer) (bFromSweep :type Boolean) (SweepResult :type "HitResult Structure (by ref)"))
  (bind _asthird_person_character (cast `ThirdPersonCharacter` OtherActor))
  (`self.SetOwner` _asthird_person_character)
  (bind _asgame_character (cast `/Game/Blueprints/Character/GameCharacter` _asthird_person_character))
  (set `self.As Game Character` _asgame_character)
  (bind _output_get (set `/Game/Blueprints/Character/GameCharacter.IsInBox` true _asgame_character))
  (`KismetSystemLibrary.PrintString` (`KismetStringLibrary.Conv_BoolToString` _output_get))
  (set `self.ExecuteLogic` true))

(event `self.Box.OnComponentEndOverlap`
  (params (OverlappedComponent :type "PrimitiveComponent Object Reference") (OtherActor :type "Actor Object Reference") (OtherComp :type "PrimitiveComponent Object Reference") (OtherBodyIndex :type Integer))
  (bind _asthird_person_character (cast `ThirdPersonCharacter` OtherActor))
  (bind _asgame_character (cast `/Game/Blueprints/Character/GameCharacter` _asthird_person_character))
  (`self.SetIsInBox_Client` false)
  (`self.SetIsInBox_Server` false)
  (set `/Game/Blueprints/Character/GameCharacter.IsInBox` false _asgame_character)
  (set `self.ExecuteLogic` false))

(event `SetIsInBox_Client`
  (params (ValueToSetTo :type Boolean))
  (set `self.IsInBox` ValueToSetTo))

(event `SetIsInBox_Server`
  (params (ValueToSetTo :type Boolean))
  (set `self.IsInBox` ValueToSetTo))

(fn `UserConstructionScript`)