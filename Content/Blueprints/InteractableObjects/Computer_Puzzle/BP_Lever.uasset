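; Interactable lever for the computer puzzle that flashes a linked Light_BP when pulled.
; A third-person character overlapping the hit box sets the lever's target rotation, and leaving resets it.
; Tick calls RotateLever and MoveHitbox, whose bodies are not shown here.
; Lever pitch reaching 55 degrees lights the lamp yellow for two seconds, then black, re-arming once pitch drops below that threshold.
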(event `self.ReceiveBeginPlay`
  (set `self.TargetRotation_0` (struct))
  (set `self.hitBoxStartLocation` (`SceneComponent.K2_GetComponentLocation` (`self.Box`))))

(event `self.ReceiveTick`
  (params (DeltaSeconds :type "Float (single-precision)"))
  (bind _lever (`self.Lever`))
  (bind (_returnvalue_roll _returnvalue_pitch) (`KismetMathLibrary.BreakRotator` (`SceneComponent.K2_GetComponentRotation` _lever)))
  (`self.rotateLever` _lever DeltaSeconds)
  (`self.moveHitbox` (`self.Box`) DeltaSeconds)
  (if (>= _returnvalue_pitch 55.0)
    (`/Engine/EditorBlueprintResources/StandardMacros.DoOnce` false :!label _label
      (:`Completed`
        (bind _aslight_bp (cast `/Game/Blueprints/InteractableObjects/Computer_Puzzle/Light_BP` (`self.lightToToggle`))
          (:`then`
            (`KismetSystemLibrary.PrintString` "Working")
            (`/Game/Blueprints/InteractableObjects/Computer_Puzzle/Light_BP.Set Lights` _aslight_bp (struct :`R` 1.0 :`G` 0.841335 :`B` 0.083688 :`A` 1.0))
            (`KismetSystemLibrary.Delay` 2.0)
            (`/Game/Blueprints/InteractableObjects/Computer_Puzzle/Light_BP.Set Lights` _aslight_bp (struct :`A` 1.0)))
          (:`CastFailed`
            (`KismetSystemLibrary.PrintString` "Not Working")))))
    (else
      (goto _label :!via `Reset`))))

(event `self.Box.OnComponentBeginOverlap`
  (params (OverlappedComponent :type "PrimitiveComponent Object Reference") (OtherActor :type "Actor Object Reference") (OtherComp :type "PrimitiveComponent Object Reference") (OtherBodyIndex :type Integer) (bFromSweep :type Boolean) (SweepResult :type "HitResult Structure (by ref)"))
  (cast `ThirdPersonCharacter` OtherActor)
  (set `self.isInBox` true)
  (set `self.targetRotation` (struct :`Pitch` 60.0)))

(event `self.Box.OnComponentEndOverlap`
  (params (OverlappedComponent :type "PrimitiveComponent Object Reference") (OtherActor :type "Actor Object Reference") (OtherComp :type "PrimitiveComponent Object Reference") (OtherBodyIndex :type Integer))
  (set `self.isInBox` false)
  (set `self.targetRotation` (struct)))

(fn `UserConstructionScript`)