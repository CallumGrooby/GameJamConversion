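; Interactable puzzle lever that sends a linked SplineWalker cart moving when the player character steps into its trigger box.
; Overlap begin and end switch the lever's target rotation between tilted and rest, while Tick calls RotateLever and MoveHitbox to update lever and box.
; A DoOnce limits MoveCart to one call per entry and re-arms when an overlap ends.
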(event `self.ReceiveBeginPlay`
  (set `self.hitBoxStartLocation` (`SceneComponent.K2_GetComponentLocation` (`self.Box`))))

(event `self.ReceiveTick`
  (params (DeltaSeconds :type "Float (single-precision)"))
  (`self.rotateLever` (`self.Lever`) DeltaSeconds)
  (`self.moveHitbox` (`self.Box`) DeltaSeconds))

(event `self.Box.OnComponentBeginOverlap`
  (params (OverlappedComponent :type "PrimitiveComponent Object Reference") (OtherActor :type "Actor Object Reference") (OtherComp :type "PrimitiveComponent Object Reference") (OtherBodyIndex :type Integer) (bFromSweep :type Boolean) (SweepResult :type "HitResult Structure (by ref)"))
  (cast `ThirdPersonCharacter` OtherActor)
  (set `self.isInBox` true)
  (set `self.targetRotation` (struct :`Pitch` 60.0))
  (`/Engine/EditorBlueprintResources/StandardMacros.DoOnce` false :!label _label
    (:`Completed`
      (`/Game/Blueprints/WirePuzzle/SplineWalker.MoveCart` (`self.SplineWalker`)))))

(event `self.Box.OnComponentEndOverlap`
  (params (OverlappedComponent :type "PrimitiveComponent Object Reference") (OtherActor :type "Actor Object Reference") (OtherComp :type "PrimitiveComponent Object Reference") (OtherBodyIndex :type Integer))
  (set `self.isInBox` false)
  (set `self.targetRotation` (struct))
  (goto _label :!via `Reset`))

(fn `UserConstructionScript`
  (`parent.UserConstructionScript`))