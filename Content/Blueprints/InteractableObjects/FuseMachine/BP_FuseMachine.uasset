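; Interactable fuse machine that pairs a fuse connection point with a lever and shows its state through a coloured light.
; On BeginPlay it hands the lever to the connection point's child fuse actor as the machine to stop, then gives the light a red dynamic material.
; RunLogic turns that material green, toggles the fuse box mesh's visibility and prints a debug string.
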(event `self.ReceiveBeginPlay`
  (bind _light2 (`self.Light2`))
  (bind _asinteractable_fuze (cast `InteractableFuze` (`ChildActorComponent.ChildActor` (`self.BP_FuzeConnectionPoint`))))
  (set `InteractableFuze.machineToStop` (`self.lever`) _asinteractable_fuze)
  (bind _returnvalue (`PrimitiveComponent.CreateDynamicMaterialInstance` _light2 0 (`PrimitiveComponent.GetMaterial` _light2 0) "Colour"))
  (`MaterialInstanceDynamic.SetVectorParameterValue` _returnvalue "Colour" (struct :`R` 1.0 :`B` 0.062529 :`A` 1.0)))

(event `self.RunLogic`
  (`KismetSystemLibrary.PrintString` "Hello")
  (`MaterialInstanceDynamic.SetVectorParameterValue` (stale `self.ReceiveBeginPlay` _returnvalue) "Colour" (struct :`G` 1.0 :`B` 0.082428 :`A` 1.0))
  (`SceneComponent.ToggleVisibility` (`self.FuseBox5`) false))

(fn `UserConstructionScript`)