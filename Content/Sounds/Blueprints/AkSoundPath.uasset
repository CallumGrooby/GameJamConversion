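; Spline-based sound path actor that calculates an occlusion value for a sound source relative to player character 0.
; OnGetOcclusionValue traces from source to player, returning zero when clear.
; If blocked, it traces to the nearest spline point: a clear path yields occlusion as interpolated fraction along the spline plus player-to-spline distance, while a blocked one yields full occlusion and a huge distance.
; Debug mode draws traces and prints partial-occlusion results.
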(event `self.ReceiveBeginPlay`
  (set `self.AudioListenerCharacter` (`GameplayStatics.GetPlayerCharacter` 0)))

(fn `OnGetOcclusionValue`
  (params (InputSoundSource :type "AkGameObject Object Reference") (DebugMode :type Boolean))
  (returns (OcculsionValueOut :type "Float (double-precision)") (isOccludedFromSpline :type Boolean) (Distance :type "Float (double-precision)"))
  (locals (hit :type "Vector Structure") (DrawMode :type "EDrawDebugTrace Enum") (DebugOn :type Boolean :default false) (OclludedFromSpline :type Boolean))
  (bind _spline (`self.Spline`))
  (bind _debugon (`local.DebugOn`))
  (bind _returnvalue (`KismetMathLibrary.TransformLocation` (`self.GetTransform` (`self.AudioListenerCharacter`))))
  (bind _returnvalue_2 (`SplineComponent.FindLocationClosestToWorldLocation` (`self.Spline`) _returnvalue "World"))
  (bind _returnvalue_3 (`KismetMathLibrary.VSize` (- _returnvalue (`local.hit`))))
  ;[1 1 1] 1. Check if player is in line of sight
  ;[1 0.6179 0.5581] Debug
  (if DebugMode
    (set `local.DrawMode` "ForOneFrame")
    (else
      (set `local.DrawMode` "None")))
  (set `local.DebugOn` DebugMode)
  (bind (_outhits _returnvalue_4) (`KismetSystemLibrary.LineTraceMulti` :`Start` (`SceneComponent.K2_GetComponentLocation` InputSoundSource) :`End` _returnvalue :`TraceChannel` "TraceTypeQuery1" :`DrawDebugType` (`local.DrawMode`) :`TraceColor` (struct :`R` 0.110933 :`G` 1.0 :`A` 1.0) :`TraceHitColor` (struct :`R` 1.0 :`G` 0.020309 :`B` 0.010362 :`A` 1.0) :`DrawTime` 0.5))
  (if _returnvalue_4
    ;[1 1 1] 2. Find Closest Point to Player
    (bind (_outhits_2 _returnvalue_5) (`KismetSystemLibrary.LineTraceMulti` :`Start` _returnvalue :`End` _returnvalue_2 :`TraceChannel` "TraceTypeQuery1" :`DrawDebugType` (`local.DrawMode`) :`TraceColor` (struct :`G` 1.0 :`B` 0.166265 :`A` 1.0) :`TraceHitColor` (struct :`R` 1.0 :`G` 0.020309 :`B` 0.010362 :`A` 1.0) :`DrawTime` 0.3))
    (if _returnvalue_5
      (bind _output_get (set `local.OclludedFromSpline` true))
      (return 1.0 _output_get 100000000.0)
      (else
        (bind _output_get_2 (set `local.hit` _returnvalue_2))
        (bind _returnvalue_6 (`SplineComponent.FindInputKeyClosestToWorldLocation` _spline _output_get_2))
        (bind _returnvalue_7 (`KismetMathLibrary.FTrunc` _returnvalue_6))
        (bind _returnvalue_8 (`SplineComponent.GetDistanceAlongSplineAtSplinePoint` (`self.Spline`) _returnvalue_7))
        (bind _returnvalue_9 (/ (+ _returnvalue_8 (* (- (`SplineComponent.GetDistanceAlongSplineAtSplinePoint` (`self.Spline`) (`KismetMathLibrary.FTrunc` (+ _returnvalue_6 1.0))) _returnvalue_8) (- _returnvalue_6 (`KismetMathLibrary.Conv_IntToDouble` _returnvalue_7)))) (`SplineComponent.GetSplineLength` _spline)))
        ;[1 1 1] 3. Find how far along spline closest point is
        (`KismetSystemLibrary.PrintString` (`KismetStringLibrary.Concat_StrStr` "Value: " (`KismetStringLibrary.Conv_DoubleToString` _returnvalue_9) " Distance: " (`KismetStringLibrary.Conv_DoubleToString` _returnvalue_3)) _debugon _debugon (struct :`R` 0.017294 :`G` 1.0 :`B` 0.920327 :`A` 1.0) 0.0)
        ;[1 1 1] 4. Return Occlusion value 0 - 1, return distance
        (return _returnvalue_9 false _returnvalue_3) ; Sound is partly occluded
      ))
    (else
      (return 0.0 false 0.0) ; Sound is not occluded
    )))

(fn `UserConstructionScript`)