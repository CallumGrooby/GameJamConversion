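; Actor component that drives custom Wwise sound occlusion for its owner, replacing the default Ak occlusion, which it switches off at BeginPlay.
; Each tick it queries every spline in its list for an occlusion value and distance, keeping the value from the nearest spline rather than the lowest value.
; That value is capped at a maximum and sent to the owner's AkGameObject as a smoothed RTPC, with optional debug printing.
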(event `self.ReceiveBeginPlay`
  (bind _returnvalue (`self.GetOwner` self))
  ;[1 1 1] Toggle Off defualt Occlusion Settings
  (`AkGameplayStatics.SetOcclusionRefreshInterval` 0.0 _returnvalue) ; Turns off Defualt Occlusion Settings
  (set `self.AkGameObject` (`Actor.GetComponentByClass` _returnvalue "/Script/AkAudio.AkGameObject")))

(event `self.ReceiveTick`
  (params (DeltaSeconds :type "Float (single-precision)"))
  (bind _drawdebugs (`self.DrawDebugs`))
  (bind _lowestocclusionvalue (`self.LowestOcclusionValue`))
  (bind _maximumocclusionvalue (`self.MaximumOcclusionValue`))
  ;[1 1 1] Loop through all Splines and find smallest occlusion value
  (set `self.LowestOcclusionValue` 1.0)
  (set `self.ShortestDistanceToSpline` 1000000000.0)
  (for _array_element (`self.List of Splines`)
    (bind (_occulsionvalueout _isoccludedfromspline _distance) (`/Game/Sounds/Blueprints/AkSoundPath.OnGetOcclusionValue` _array_element (`self.AkGameObject`) (`self.DrawDebugs`))) ; Does math for each spline
    (if (< _distance (`self.ShortestDistanceToSpline`))
      (set `self.LowestOcclusionValue` _occulsionvalueout)
      (set `self.ShortestDistanceToSpline` _distance)))
  ;[1 1 1] Set Occlusion
  (if (> (`self.LowestOcclusionValue`) _maximumocclusionvalue)
    (set `self.LowestOcclusionValue` _maximumocclusionvalue))
  (`AkGameObject.SetRTPCValue` (`self.AkGameObject`) "/Game/WwiseAudio/Game_Parameters/Default_Work_Unit/CustomOcclusionValueRTPC.CustomOcclusionValueRTPC" _lowestocclusionvalue 300 "") ; Set RTPC Occlusion value for that Object
  (`KismetSystemLibrary.PrintString` (`KismetStringLibrary.Concat_StrStr` "Lowest Occlusion value == " (`KismetStringLibrary.Conv_DoubleToString` _lowestocclusionvalue)) _drawdebugs _drawdebugs (struct :`R` 1.0 :`G` 1.0 :`B` 1.0 :`A` 1.0) 0.0))